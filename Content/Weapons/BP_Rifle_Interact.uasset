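; A rifle pickup actor that swaps itself for an equipped rifle when the player presses E while looking at it.
; A camera-forward visibility trace must hit this actor, and the player character must be within close range.
; It then spawns BP_Rifle_Connect owned by the player, snaps it to the mesh's hand_r socket, and destroys itself once attachment succeeds.
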(event Input|KeyboardEvents|E
  (params (Key :type Key%20Structure :default "None"))
  (bind _returnvalue (Game|GetPlayerCharacter 0))
  (bind _returnvalue_2 (Game|GetPlayerCameraManager 0))
  (bind _returnvalue_3 (Camera|GetCameraLocation _returnvalue_2))
  (bind _mesh (Variables|/Script/Engine.Character|GetMesh _returnvalue))
  (:Pressed
    (bind _outhit (Collision|LineTraceByChannel _returnvalue_3 (+ _returnvalue_3 (* (Math|Vector|GetForwardVector (Camera|GetCameraRotation _returnvalue_2)) "2000,2000,2000")) "TraceTypeQuery1" false (Utilities|Array|MakeArray _returnvalue) "None" false))
    (if (== (.HitActor (Collision|BreakHitResult _outhit)) self)
      (if (<= (Transformation|GetDistanceTo _returnvalue) 2e+02)
        (if (Transformation|DoesSocketExist _mesh "hand_r")
          (bind _returnvalue_4 (Game|SpawnActorfromClass "/Game/Weapons/BP_Rifle_Connect.BP_Rifle_Connect_C" (Math|Transform|MakeTransform "0, 0, 0") "AlwaysSpawn" "MultiplyWithRoot" _returnvalue 0))
          (Utilities|IsValid _returnvalue_4
            (:Is%20Valid
              (bind _returnvalue_5 (Transformation|AttachComponentToComponent _returnvalue_4 _mesh "hand_r" "SnapToTarget" "SnapToTarget" "KeepWorld" false))
              (if _returnvalue_5
                (Actor|DestroyActor)))))))))

(fn ConstructionScript)